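; Character component for Base_Character that lets the player target and loot resources and holds a capped resource stock.
; A looping timer drives a trace from the camera to the character's hit location, tracking the Int_Lootable actor under it and sending hover and leave messages.
; Pressing E sends that actor a loot message if within range, with debug prints.
; AddRessourceToStock adds to the stock, clamped to its maximum.
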(event `self.ReceiveBeginPlay`
  (`|ExecutionSequence`
    (:`then_0`
      (bind _asbase_character (cast `/Game/Blueprints/Gameplay/Base_Character` (`self.GetOwner`)))
      (set `self.As Character` _asbase_character))
    (:`then_1`
      (`KismetSystemLibrary.K2_SetTimerDelegate` (`|CreateDelegate` :!event `CheckLootableRessources`) 0.1 true))))

(event `CheckLootableRessources`
  (bind _lasthitlootable (`self.LastHitLootable`))
  (bind _outhit (`KismetSystemLibrary.LineTraceSingleForObjects` (`PlayerCameraManager.GetCameraLocation` (`PlayerController.PlayerCameraManager` (`GameplayStatics.GetPlayerController` 0))) (`/Game/Blueprints/Gameplay/Base_Character.Hit Result Location` (`self.As Character`)) (`|MakeArray` "ObjectTypeQuery1" "ObjectTypeQuery2" :!type "EObjectTypeQuery Enum")))
  (bind (_bblockinghit _binitialoverlap _time _distance _location _impactpoint _normal _impactnormal _physmat _hitactor) (`GameplayStatics.BreakHitResult` _outhit))
  (if (`KismetSystemLibrary.DoesImplementInterface` _hitactor "/Game/Blueprints/Gameplay/AC_RessourceGathering/Int_Lootable.Int_Lootable_C")
    (bind _output_get (set `self.LastHitLootable` _hitactor))
    (message `/Game/Blueprints/Gameplay/AC_RessourceGathering/Int_Lootable.OnMouseOver` _output_get)
    (else
      (`/Engine/EditorBlueprintResources/StandardMacros.IsValid` _lasthitlootable
        (:`Is Valid`
          (message `/Game/Blueprints/Gameplay/AC_RessourceGathering/Int_Lootable.OnMouseLeave` _lasthitlootable)
          (set `self.LastHitLootable` null))))))

(event `Key|E`
  (params (Key :type "Key Structure"))
  (bind _lasthitlootable (`self.LastHitLootable`))
  (:`Pressed`
    (`/Engine/EditorBlueprintResources/StandardMacros.IsValid` _lasthitlootable
      (:`Is Valid`
        (if (< (`KismetMathLibrary.Vector_Distance2D` (`Actor.K2_GetActorLocation` _lasthitlootable) (`Actor.K2_GetActorLocation` (`self.As Character`))) 500.0)
          (message `/Game/Blueprints/Gameplay/AC_RessourceGathering/Int_Lootable.OnLoot` _lasthitlootable)
          (`KismetSystemLibrary.PrintString` (`KismetStringLibrary.Conv_IntToString` (`self.CurrentStockValue`)))
          (else
            (`KismetSystemLibrary.PrintString` "The loot is too far")))))))

(fn `AddRessourceToStock`
  (params (Value :type Integer))
  (set `self.CurrentStockValue` (`KismetMathLibrary.Clamp` (+ (`self.CurrentStockValue`) Value) 0 (`self.MaxStockValue`)))
  (return))