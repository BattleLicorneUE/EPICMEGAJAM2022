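; Health component for a Character owner, storing health, max and god mode in a struct, with clamped damage, healing and percent queries.
; ApplyDamages respects god mode, returns true on death, and otherwise plays a random hit montage, gated by a DoOnce until it ends.
; ApplyDamagesMagic ignores god mode, calls DeathCharacter on player 0's Base_Character at zero health regardless of owner, and otherwise plays a 2D sound.
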(event `self.ReceiveBeginPlay`
  (bind _ascharacter (cast `Character` (`self.GetOwner`)))
  (set `self.Owner` _ascharacter))

(event `Play Hit Montage`
  (`/Engine/EditorBlueprintResources/StandardMacros.DoOnce` false :!label _label
    (:`Completed`
      (`|PlayMontage` (`Character.Mesh` (`self.Owner`)) (`KismetArrayLibrary.Array_Random` (`self.Hit Montage`))
        (:`OnCompleted`
          (goto _label :!via `Reset`))
        (:`OnBlendOut`
          (goto _label :!via `Reset`))
        (:`OnInterrupted`
          (`KismetSystemLibrary.Delay` 1.0)
          (goto _label :!via `Reset`))))))

(fn `Add Heath`
  (params (`Add Health` :type "Float (double-precision)"))
  (bind (_health _healthmax) (break `/Game/Blueprints/Gameplay/AC_Health/S_Struct_Health` (`self.S_Health`)))
  (setmembers `/Game/Blueprints/Gameplay/AC_Health/S_Struct_Health` :`StructRef` (`self.S_Health`) :`Health` (`KismetMathLibrary.FClamp` (+ `Add Health` _health) 0.0 _healthmax)))

(fn `Apply Damages`
  (params (Damages :type "Float (double-precision)"))
  (returns (`Actor is Dead` :type Boolean))
  (bind _s_health (`self.S_Health`))
  (bind (_health _healthmax _godmod) (break `/Game/Blueprints/Gameplay/AC_Health/S_Struct_Health` _s_health))
  (if (not _godmod)
    (bind _structout (setmembers `/Game/Blueprints/Gameplay/AC_Health/S_Struct_Health` :`StructRef` _s_health :`Health` (`KismetMathLibrary.FClamp` (- _health Damages) 0.0 _healthmax)))
    (if (<= (break `/Game/Blueprints/Gameplay/AC_Health/S_Struct_Health` _structout) 0.0)
      (return true)
      (else
        (`self.Play Hit Montage`)
        (return false)))))

(fn `Apply Damages Magic`
  (params (Damages :type "Float (double-precision)"))
  (bind _s_health (`self.S_Health`))
  (bind (_health _healthmax) (break `/Game/Blueprints/Gameplay/AC_Health/S_Struct_Health` _s_health))
  (bind _structout (setmembers `/Game/Blueprints/Gameplay/AC_Health/S_Struct_Health` :`StructRef` _s_health :`Health` (`KismetMathLibrary.FClamp` (- _health Damages) 0.0 _healthmax)))
  (if (<= (break `/Game/Blueprints/Gameplay/AC_Health/S_Struct_Health` _structout) 0.0)
    (bind _asbase_character (cast `/Game/Blueprints/Gameplay/Base_Character` (`GameplayStatics.GetPlayerCharacter` 0)))
    (`/Game/Blueprints/Gameplay/Base_Character.Death Character` _asbase_character)
    (else
      (`GameplayStatics.PlaySound2D` null 1.0 1.0 0.0 null null))))

(fn `Get Percent`
  (returns (`Get Percent` :type "Float (double-precision)"))
  (bind (_health _healthmax) (break `/Game/Blueprints/Gameplay/AC_Health/S_Struct_Health` (`self.S_Health`)))
  (return (/ _health _healthmax)))