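; Actor component that performs the player's spell attack on its owning Base_Character.
; ATK plays a random attack montage at double speed, gated by a DoOnce that resets only when the montage completes.
; Montage notifies drive the effects: Spawn launches a BP_ProjectileMaster from the right-hand point toward the owner's HitResultLocation, and Spawn VFX places a Niagara magic circle.
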(event `self.ReceiveBeginPlay`
  (bind _asbase_character (cast `/Game/Blueprints/Gameplay/Base_Character` (`self.GetOwner`)))
  (set `self.Owner` _asbase_character))

(event `ATK`
  (bind _owner (`self.Owner`))
  (bind _returnvalue (`SceneComponent.K2_GetComponentLocation` (`/Game/Blueprints/Gameplay/Base_Character.SpawnProjectileHandR` _owner)))
  (`/Engine/EditorBlueprintResources/StandardMacros.DoOnce` false :!label _label
    (:`Completed`
      (bind _notifyname (`|PlayMontage` (`Character.Mesh` (`self.Owner`)) (`KismetArrayLibrary.Array_Random` (`self.Montage to Play ATK`)) 2.0)
        (:`OnCompleted`
          (goto _label :!via `Reset`))
        (:`OnNotifyBegin`
          (switch `name` _notifyname
            (:`Spawn`
              (`|SpawnActorFromClass` "/Game/Blueprints/Gameplay/BP_ProjectileMaster.BP_ProjectileMaster_C" (`KismetMathLibrary.MakeTransform` _returnvalue (`KismetMathLibrary.FindLookAtRotation` _returnvalue (`/Game/Blueprints/Gameplay/Base_Character.Hit Result Location` _owner))) "AdjustIfPossibleButAlwaysSpawn" "OverrideRootScale" null null))
            (:`SpawnVFX`
              (`NiagaraFunctionLibrary.SpawnSystemAtLocation` "/Game/VFX/NS_CercleMagic.NS_CercleMagic" (`SceneComponent.K2_GetComponentLocation` (`/Game/Blueprints/Gameplay/Base_Character.SpawnCercleMagic` _owner))))))))))