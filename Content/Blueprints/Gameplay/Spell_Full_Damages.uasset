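; Area damage spell actor that hurts every AI overlapping it when its ApplyDamages event fires.
; The event shakes the first player's camera and plays an air spell sound, then applies flat damage to each overlapping BP_AI_Master.
; Each hit also spawns a Niagara impact at the Scene component and an ice impact sound at the spell's location, rather than on the target.
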(event `Apply Damages`
  (`PlayerController.ClientStartCameraShake` :`self` (`GameplayStatics.GetPlayerController` 0) :`Shake` "/Game/Feedback/CameraShakes/CS_Weapon_Fire_Explosion.CS_Weapon_Fire_Explosion_C")
  (`GameplayStatics.PlaySoundAtLocation` "/Game/Sounds/4_elements_spells/Cues/Spell_Air_04_Cue.Spell_Air_04_Cue" (`self.K2_GetActorLocation`) (struct) 1.0 1.0 0.0 "/Game/Sounds/NaturalSoundAttenuation.NaturalSoundAttenuation" null null null)
  (for _array_element (`self.GetOverlappingActors` "/Game/Blueprints/Gameplay/AI/BP_AI_Master.BP_AI_Master_C")
    (`GameplayStatics.ApplyDamage` _array_element 100.0)
    (`NiagaraFunctionLibrary.SpawnSystemAtLocation` "/Game/VFX/Explosion/NS_HitEnvironement.NS_HitEnvironement" (`SceneComponent.K2_GetComponentLocation` (`self.Scene`)))
    (`GameplayStatics.PlaySoundAtLocation` "/Game/Sounds/4_elements_spells/Cues/Spell_Ice_Impact_Critical_Cue.Spell_Ice_Impact_Critical_Cue" (`self.K2_GetActorLocation`) (struct) 1.0 1.0 0.0 "/Game/Sounds/NaturalSoundAttenuation.NaturalSoundAttenuation" null null null)))

(fn `UserConstructionScript`)