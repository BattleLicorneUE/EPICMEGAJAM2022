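; AC_Mana is an actor component that manages a mana pool stored in a struct.
; It adds and spends mana clamped between zero and the maximum, and reports the current fraction.
; Check Mana spends the cost when affordable; otherwise it empties the pool and applies the full cost as magic damage to the first player character's AC_Health component.
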(fn `Add Mana`
  (params (`Add Mana` :type "Float (double-precision)"))
  (bind (_manacurrent _manamax) (break `/Game/Blueprints/Gameplay/AC_Mana/S_Mana` (`self.Mana`)))
  (setmembers `/Game/Blueprints/Gameplay/AC_Mana/S_Mana` :`StructRef` (`self.Mana`) :`Mana Current` (`KismetMathLibrary.FClamp` (+ `Add Mana` _manacurrent) 0.0 _manamax)))

(fn `Check Mana`
  (params (A :type "Float (double-precision)"))
  (bind _mana_manacurrent (break `/Game/Blueprints/Gameplay/AC_Mana/S_Mana` (`self.Mana`)))
  (if (<= A _mana_manacurrent)
    (`self.Use Mana` A)
    (return)
    (else
      (setmembers `/Game/Blueprints/Gameplay/AC_Mana/S_Mana` :`StructRef` (`self.Mana`) :`Mana Current` 0.0)
      (`/Game/Blueprints/Gameplay/AC_Health/AC_Health.Apply Damages Magic` (`Actor.GetComponentByClass` (`GameplayStatics.GetPlayerCharacter` 0) "/Game/Blueprints/Gameplay/AC_Health/AC_Health.AC_Health_C") A)
      (return))))

(fn `Get Percent`
  (returns (ReturnValue :type "Float (double-precision)"))
  (bind (_mana_manacurrent _mana_manamax) (break `/Game/Blueprints/Gameplay/AC_Mana/S_Mana` (`self.Mana`)))
  (return (/ _mana_manacurrent _mana_manamax)))

(fn `Use Mana`
  (params (`Mana Requis` :type "Float (double-precision)"))
  (bind (_manacurrent _manamax) (break `/Game/Blueprints/Gameplay/AC_Mana/S_Mana` (`self.Mana`)))
  (setmembers `/Game/Blueprints/Gameplay/AC_Mana/S_Mana` :`StructRef` (`self.Mana`) :`Mana Current` (`KismetMathLibrary.FClamp` (- _manacurrent `Mana Requis`) 0.0 _manamax)))