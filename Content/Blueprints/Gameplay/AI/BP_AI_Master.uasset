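; Master AI character Blueprint that handles damage, health display and death.
; Damage goes to ACHealth; non-lethal hits update the WB_AI_HealthInfo widget, briefly show it via a retriggerable delay, and set a BP_AIController state.
; Each state change targets player character 0, whoever dealt the damage.
; Death runs once: it changes state, ragdolls the mesh, removes the light and capsule collision, plays a sound, then destroys the actor after a delay.
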(event `self.ReceiveBeginPlay`
  (`self.Update Widget Health`))

(event `self.ReceiveAnyDamage`
  (params (Damage :type "Float (single-precision)") (DamageType :type "DamageType Object Reference") (InstigatedBy :type "Controller Object Reference") (DamageCauser :type "Actor Object Reference"))
  (bind _actor_is_dead (`/Game/Blueprints/Gameplay/AC_Health/AC_Health.Apply Damages` (`self.AC_Health`) Damage))
  (if _actor_is_dead
    (`/Engine/EditorBlueprintResources/StandardMacros.DoOnce` false
      (:`Completed`
        (`self.Set AI State` "NewEnumerator3")
        (`self.SetSimulateRadgoll`)
        (`self.SetVisibleHealth` false)
        (`GameplayStatics.PlaySoundAtLocation` "/Game/Sounds/SoundsCue_Perso/Death.Death" (`self.K2_GetActorLocation`) (struct) 1.0 1.0 0.0 "/Game/Sounds/NaturalSoundAttenuation.NaturalSoundAttenuation" null null null)
        (`KismetSystemLibrary.Delay` 10.0)
        (`self.K2_DestroyActor`)))
    (else
      (`self.Update Widget Health`)
      (`self.Set AI State` "NewEnumerator2")
      (if (not (`self.Dead`))
        (`self.SetVisibleHealth` true)
        (`KismetSystemLibrary.RetriggerableDelay` 5.0)
        (`self.SetVisibleHealth` false)))))

(fn `Set AI State`
  (params (State_AI :type "/Game/Blueprints/Gameplay/AI/AI_Complexe/E_State_AI Enum" :default "NewEnumerator0"))
  (bind _asbp_aicontroller (cast `/Game/Blueprints/Gameplay/AI/AI_Complexe/BP_AIController` (`AIBlueprintHelperLibrary.GetAIController` self)))
  (`/Game/Blueprints/Gameplay/AI/AI_Complexe/BP_AIController.Set State AI` _asbp_aicontroller State_AI)
  (`/Game/Blueprints/Gameplay/AI/AI_Complexe/BP_AIController.Set Target` _asbp_aicontroller (`GameplayStatics.GetPlayerCharacter` 0)))

(fn `SetSimulateRadgoll`
  (set `self.Dead` true)
  (`ActorComponent.K2_DestroyComponent` (`self.PointLight`))
  (`PrimitiveComponent.SetSimulatePhysics` (`self.Mesh`) true)
  (`PrimitiveComponent.SetCollisionEnabled` (`self.CapsuleComponent`) "NoCollision"))

(fn `SetVisibleHealth`
  (params (bNewVisibility :type Boolean))
  (`SceneComponent.SetVisibility` (`self.Widget_Health`) bNewVisibility false))

(fn `Update Widget Health`
  (bind _aswb_ai_health_info (cast `/Game/Blueprints/Gameplay/AI/WB_AI_HealthInfo` (`WidgetComponent.GetUserWidgetObject` (`self.Widget_Health`))))
  (set `/Game/Blueprints/Gameplay/AI/WB_AI_HealthInfo.Health` (`/Game/Blueprints/Gameplay/AC_Health/AC_Health.Get Percent` (`self.AC_Health`)) _aswb_ai_health_info))

(fn `UserConstructionScript`)