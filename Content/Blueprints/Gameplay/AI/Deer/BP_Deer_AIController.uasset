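; AI controller for the deer that starts its behavior tree and switches its movement between a slow and a fast speed.
; On possessing an AI_Deer pawn, it caches the deer, runs DeerBehaviorTree and sets the slow max walk speed.
; AI Perception updates raise the speed for any Character and restore it for other actors, without checking whether the stimulus was sensed or lost.
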(event `self.ReceivePossess`
  (params (PossessedPawn :type "Pawn Object Reference"))
  (bind _asai_deer (cast `/Game/Blueprints/Gameplay/AI/Deer/AI_Deer` PossessedPawn))
  (set `self.As AI Deer` _asai_deer)
  (`self.RunBehaviorTree` "/Game/Blueprints/Gameplay/AI/Deer/DeerBehaviorTree.DeerBehaviorTree")
  (set `CharacterMovementComponent.MaxWalkSpeed` 200.0 (`Character.CharacterMovement` (`self.As AI Deer`))))

(event `self.AIPerception.OnTargetPerceptionUpdated`
  (params (Actor :type "Actor Object Reference") (Stimulus :type "AIStimulus Structure"))
  (bind _charactermovement (`Character.CharacterMovement` (`self.As AI Deer`)))
  (cast `Character` Actor
    (:`then`
      (set `CharacterMovementComponent.MaxWalkSpeed` 600.0 _charactermovement))
    (:`CastFailed`
      (set `CharacterMovementComponent.MaxWalkSpeed` 200.0 _charactermovement))))

(fn `UserConstructionScript`)