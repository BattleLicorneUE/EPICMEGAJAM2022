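; BP_BOOK_Life is a pickup book that restores health to a character that touches it.
; Its sphere overlap casts the other actor to Base_Character and runs once through a DoOnce, adding AddHealth to that character's ACHealth component.
; It then spawns a green magic-circle Niagara effect, plays a heal camera shake on player controller 0 and a spatialized buff sound, and destroys itself.
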(event `self.Sphere.OnComponentBeginOverlap`
  (params (OverlappedComponent :type "PrimitiveComponent Object Reference") (OtherActor :type "Actor Object Reference") (OtherComp :type "PrimitiveComponent Object Reference") (OtherBodyIndex :type Integer) (bFromSweep :type Boolean) (SweepResult :type "HitResult Structure (by ref)"))
  (bind _asbase_character (cast `/Game/Blueprints/Gameplay/Base_Character` OtherActor))
  (`/Engine/EditorBlueprintResources/StandardMacros.DoOnce` false
    (:`Completed`
      (`/Game/Blueprints/Gameplay/AC_Health/AC_Health.Add Heath` (`/Game/Blueprints/Gameplay/Base_Character.AC_Health` _asbase_character) (`self.Add Health`))
      (`NiagaraFunctionLibrary.SpawnSystemAtLocation` "/Game/VFX/CercleMagic/NS_CercleMagic_Green.NS_CercleMagic_Green" (`self.K2_GetActorLocation`))
      (`PlayerController.ClientStartCameraShake` :`self` (`GameplayStatics.GetPlayerController` 0) :`Shake` "/Game/Feedback/CameraShakes/CS_Character_Heal.CS_Character_Heal_C")
      (`GameplayStatics.PlaySoundAtLocation` "/Game/Sounds/4_elements_spells/Cues/Spell_Air_Buff_Cue.Spell_Air_Buff_Cue" (`self.K2_GetActorLocation`) (struct) 1.0 1.0 0.0 "/Game/Sounds/NaturalSoundAttenuation.NaturalSoundAttenuation" null null null)
      (`self.K2_DestroyActor`))))

(fn `UserConstructionScript`)