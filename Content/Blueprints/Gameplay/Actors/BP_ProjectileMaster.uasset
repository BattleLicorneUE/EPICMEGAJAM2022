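; BP_ProjectileMaster is a projectile actor that deals radial damage on impact, sparing its DamageCauser and crediting that causer's instigator controller.
; The sphere's hit event applies the damage, then calls PlayFeedback with the character-hit effect regardless of what was struck.
; PlayFeedback spawns the effect, shakes player 0's camera, plays a fixed sound for Character hits or a random HitSound otherwise, then destroys the projectile.
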(event `self.Sphere.OnComponentHit`
  (params (HitComponent :type "PrimitiveComponent Object Reference") (OtherActor :type "Actor Object Reference") (OtherComp :type "PrimitiveComponent Object Reference") (NormalImpulse :type "Vector Structure") (Hit :type "HitResult Structure (by ref)"))
  (bind _damage_causer (`self.Damage Causer`))
  (`GameplayStatics.ApplyRadialDamage` 30.0 (`.Location` (`GameplayStatics.BreakHitResult` Hit)) 200.0 null (`|MakeArray` _damage_causer) _damage_causer (`self.GetInstigatorController` _damage_causer))
  (`self.Play Feedback` Hit (`self.System Template hit Character`)))

(fn `Play Feedback`
  (params (Hit :type "HitResult Structure (by ref)") (SystemTemplate :type "NiagaraSystem Object Reference"))
  (bind (_bblockinghit _binitialoverlap _time _distance _location _impactpoint _normal _impactnormal _physmat _hitactor) (`GameplayStatics.BreakHitResult` Hit))
  (bind _outitem (`KismetArrayLibrary.Array_Random` (`self.Hit Sound`)))
  (`NiagaraFunctionLibrary.SpawnSystemAtLocation` SystemTemplate _location)
  (`PlayerController.ClientStartCameraShake` :`self` (`GameplayStatics.GetPlayerController` 0) :`Shake` "/Game/Feedback/CameraShakes/CS_Character_DamageTaken.CS_Character_DamageTaken_C")
  (cast `Character` _hitactor
    (:`then`
      (`GameplayStatics.PlaySoundAtLocation` "/Game/Sounds/4_elements_spells/Cues/Shield_Ice_Cue.Shield_Ice_Cue" (`self.K2_GetActorLocation`) (struct) 1.0 1.0 0.0 "/Game/Sounds/NaturalSoundAttenuation.NaturalSoundAttenuation" null null null))
    (:`CastFailed`
      (`/Engine/EditorBlueprintResources/StandardMacros.IsValid` _outitem
        (:`Is Valid`
          (`GameplayStatics.PlaySoundAtLocation` _outitem _location (struct) 1.0 1.0 0.0 "/Game/Sounds/NaturalSoundAttenuation.NaturalSoundAttenuation" null null null))
        (:`Is Not Valid`
          _))))
  (`self.K2_DestroyActor`))

(fn `UserConstructionScript`)